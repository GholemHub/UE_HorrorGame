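; A usable radio actor that toggles its sound on and off when the player uses it.
; Use prints a debug string and runs a FlipFlop: one branch starts RadioSound through ReplaceRadioSound, replacing any sound in NowPlay.
; The other branch stops the managed sound held in NowPlay.
; A separate OnRadio event also starts the sound directly.
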(event `OnRadio`
  (bind _returnvalue (`self.ReplaceRadioSound` (`self.NowPlay`) (`self.RadioSound`) :!label _label))
  (set `self.NowPlay` _returnvalue))

(event `self.Use`
  (params (Character :type "Actor Object Reference"))
  (`KismetSystemLibrary.PrintString` "Hello")
  (`self.On/OfRadio`))

(event `On/OfRadio`
  (bind _nowplay (`self.NowPlay`))
  (`/Engine/EditorBlueprintResources/StandardMacros.FlipFlop`
    (:`A`
      (goto _label))
    (:`B`
      (`/Engine/EditorBlueprintResources/StandardMacros.IsValid` _nowplay
        (:`Is Valid`
          (`HronoAudioLibrary.StopManagedSound` _nowplay))))))

(fn `UserConstructionScript`)