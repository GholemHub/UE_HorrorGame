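; BP_Clock_Item is a usable clock item Blueprint whose Tick and Use events are currently empty.
; Disconnected nodes remain for rotating a component, either by setting pitch from TimeNow or stepping it each call, with a different delta when IsCursed is set.
; Other unreachable nodes play a ClockReset sound at the actor and print TimeNow, so the graph has no active behavior.
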(event `self.ReceiveTick`
  (params (DeltaSeconds :type "Float (single-precision)")))

(event `self.Use`
  (params (Character :type "Actor Object Reference")))

(fn `UserConstructionScript`)