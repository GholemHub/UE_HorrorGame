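; BP_TriggerBox is a trigger volume that sets off a scare when an HE_CharacterHrono1 overlaps its box.
; Each overlap notifies the linked ATriggerActor, then asks it whether the character's timeline matches.
; On a match, only the server calls ScareEvent on the character, guarded by a DoOnce so it fires a single time.
; The local OnSameTimeline function is a stub returning false, and a Delay node is left unconnected.
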(event `self.ReceiveBeginPlay`)

(event `self.Box.OnComponentBeginOverlap`
  (params (OverlappedComponent :type "PrimitiveComponent Object Reference") (OtherActor :type "Actor Object Reference") (OtherComp :type "PrimitiveComponent Object Reference") (OtherBodyIndex :type Integer) (bFromSweep :type Boolean) (SweepResult :type "HitResult Structure (by ref)"))
  (bind _ashe_character_hrono_1 (cast `/Game/_Alex/HE_CharacterHrono1` OtherActor))
  (`/Engine/EditorBlueprintResources/StandardMacros.IsValid` (`self.ATriggerActor`)
    (:`Is Valid`
      (message `/Game/_Alex/I_ScareInterface.OnScareTrigger` (`self.ATriggerActor`) _ashe_character_hrono_1)
      (bind _hassametimelines (message `/Game/_Alex/I_ScareInterface.OnSameTimeline` (`self.ATriggerActor`) (`HronoCharacter.CharacterTimeline` _ashe_character_hrono_1)))
      (if _hassametimelines
        (`/Engine/EditorBlueprintResources/ActorMacros.Switch Has Authority`
          (:`Authority`
            (`/Engine/EditorBlueprintResources/StandardMacros.DoOnce` false
              (:`Completed`
                (`/Game/_Alex/HE_CharacterHrono1.ScareEvent` _ashe_character_hrono_1)))))))))

(fn `OnSameTimeline`
  (params (CharacterTimeline :type "EItemTimeline Enum" :default "Past"))
  (returns (HasSameTimelines :type Boolean))
  (return false))

(fn `UserConstructionScript`)