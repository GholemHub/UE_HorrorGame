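; BP_ScareActor is a one-shot scare prop that lunges along world X when triggered, then destroys itself.
; OnscareTrigger fires only if the triggerer's CharacterTimeline matches the actor's ItemTimeline, repeating the check OnSameTimeline offers.
; A Timeline lerps from the current location toward a positive X offset, both re-read each update, so movement accumulates.
; The Trigger function is an empty stub.
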(event `/Game/_Alex/I_ScareInterface.OnscareTrigger`
  (params (Triggerer :type "/Game/_Alex/HE_CharacterHrono1 Object Reference"))
  (bind (_returnvalue_x _returnvalue_y _returnvalue_z) (`KismetMathLibrary.BreakVector` (`self.K2_GetActorLocation`)))
  (if (`|EnumEquality` (`HronoCharacter.CharacterTimeline` Triggerer) (`self.ItemTimeline`))
    (bind (_direction _newtrack_0) (`Timeline|Timeline_0` :!via `PlayFromStart`)
      (:`Update`
        (`self.K2_SetActorLocation` (`KismetMathLibrary.VLerp` (`self.K2_GetActorLocation`) (`KismetMathLibrary.MakeVector` (- _returnvalue_x -40.0) _returnvalue_y _returnvalue_z) _newtrack_0)))
      (:`Finished`
        (`self.K2_DestroyActor`)))))

(fn `OnSameTimeline`
  (params (CharacterTimeline :type "EItemTimeline Enum" :default "Past"))
  (returns (HasSameTimelines :type Boolean))
  (return (`|EnumEquality` CharacterTimeline (`self.ItemTimeline`))))

(fn `Trigger`
  (params (Triggerer :type "/Game/_Alex/HE_CharacterHrono1 Object Reference")))

(fn `UserConstructionScript`)