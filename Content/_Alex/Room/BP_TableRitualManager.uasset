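; Table ritual manager that runs a two-player séance-style sequence with chairs, candles, a bottle and a board.
; StartRitual requires both chairs occupied, then uses random delays to nudge the ritual chair with a creak, light candles and spin the bottle on authority.
; VictimChoise turns the board toward the victim and curses that sitter on authority.
; NextTryRitual triggers a candle mistake and respin, or the board's goodbye when lives run out.
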(event `self.Box.OnComponentBeginOverlap`
  (params (OverlappedComponent :type "PrimitiveComponent Object Reference") (OtherActor :type "Actor Object Reference") (OtherComp :type "PrimitiveComponent Object Reference") (OtherBodyIndex :type Integer) (bFromSweep :type Boolean) (SweepResult :type "HitResult Structure (by ref)")))

(event `self.Box.OnComponentEndOverlap`
  (params (OverlappedComponent :type "PrimitiveComponent Object Reference") (OtherActor :type "Actor Object Reference") (OtherComp :type "PrimitiveComponent Object Reference") (OtherBodyIndex :type Integer)))

(event `StartRitual`
  (bind _ritualchair (`self.RitualChair`))
  (bind _returnvalue (`self.K2_GetActorLocation` _ritualchair))
  (if (`self.bIsFirstAttempt`)
    (if (and (`Chair.bIsSit` (`self.Chair1`)) (`Chair.bIsSit` (`self.Chair2`)))
      (`/Game/_Alex/Usable/BP_Chair.StartRitual` (`self.Chair1`))
      (`/Game/_Alex/Usable/BP_Chair.StartRitual` (`self.Chair2`))
      (`KismetSystemLibrary.Delay` (`KismetMathLibrary.RandomFloatInRange` 1.0 3.0))
      (set `self.bIsFirstAttempt` false)
      (`/Engine/EditorBlueprintResources/StandardMacros.IsValid` (`self.RitualChair`)
        (:`Is Valid`
          (bind (_direction _newtrack_0) (`Timeline|Timeline` :!via `PlayFromStart`)
            (:`Update`
              (`/Engine/EditorBlueprintResources/ActorMacros.Switch Has Authority`
                (:`Authority`
                  (bind _returnvalue_2 (`KismetMathLibrary.VLerp` _returnvalue (- _returnvalue (* (`self.GetActorForwardVector` _ritualchair) 0.2)) _newtrack_0))
                  (`self.K2_SetActorLocation` _ritualchair _returnvalue_2 false false)
                  (`/Engine/EditorBlueprintResources/StandardMacros.DoOnce` false
                    (:`Completed`
                      (`GameplayStatics.PlaySoundAtLocation` "/Game/HorrorEngine/Audio/Interactions/S_Creak_06.S_Creak_06" _returnvalue_2 (struct) 1.0 1.0 0.0 null null null null))))))
            (:`Finished`
              (`KismetSystemLibrary.Delay` (`KismetMathLibrary.RandomFloatInRange` 1.0 3.0))
              (`/Game/_Alex/Pickable/BP_Item_Candle.LightAll` (`self.Candle`) 0)
              (`KismetSystemLibrary.Delay` (`KismetMathLibrary.RandomFloatInRange` 3.0 5.0))
              (`/Engine/EditorBlueprintResources/ActorMacros.Switch Has Authority`
                (:`Authority`
                  (`RitualBottle.SpinBottle` (`self.Bottle`) (`Chair.GetSitter` (`self.Chair2`)) (`Chair.GetSitter` (`self.Chair1`)))))))))
      (else
        (`KismetSystemLibrary.PrintString` "NotSite")))))

(event `VictimChoise`
  (params (Victim :type Boolean))
  (bind _board (`self.Board`))
  (bind _board_2 (`self.Board`))
  (bind _returnvalue (`Chair.GetSitter` (`self.Chair2`)))
  (bind _returnvalue_2 (`Chair.GetSitter` (`self.Chair1`)))
  (bind (_returnvalue_roll _returnvalue_pitch) (`KismetMathLibrary.BreakRotator` (`self.K2_GetActorRotation` _board_2)))
  (bind (_returnvalue_roll_2 _returnvalue_pitch_2) (`KismetMathLibrary.BreakRotator` (`self.K2_GetActorRotation` _board)))
  (`/Engine/EditorBlueprintResources/ActorMacros.Switch Has Authority`
    (:`Authority`
      (`self.SetActorHiddenInGame` (`self.Board`) false)
      (if Victim
        (`self.K2_SetActorRotation` _board_2 (`KismetMathLibrary.MakeRotator` _returnvalue_roll _returnvalue_pitch 180.0) false)
        (else
          (`self.K2_SetActorRotation` _board (`KismetMathLibrary.MakeRotator` _returnvalue_roll_2 _returnvalue_pitch_2) false)))
      (`KismetSystemLibrary.Delay` 2.0)
      (if Victim
        (`/Engine/EditorBlueprintResources/StandardMacros.IsValid` _returnvalue_2
          (:`Is Valid`
            (bind _ashe_character_hrono_1 (cast `/Game/_Alex/HE_CharacterHrono1` _returnvalue_2))
            (`/Game/_Alex/HE_CharacterHrono1.VictimCurse` _ashe_character_hrono_1)))
        (else
          (`/Engine/EditorBlueprintResources/StandardMacros.IsValid` _returnvalue
            (:`Is Valid`
              (bind _ashe_character_hrono_1_2 (cast `/Game/_Alex/HE_CharacterHrono1` _returnvalue))
              (`/Game/_Alex/HE_CharacterHrono1.VictimCurse` _ashe_character_hrono_1_2))))))))

(event `Test`
  (`KismetSystemLibrary.Delay` (`KismetMathLibrary.RandomFloatInRange` 1.0 3.0) :!label _label)
  (`/Game/_Alex/Pickable/BP_Item_Candle.OnMistake` (`self.Candle`))
  (`KismetSystemLibrary.Delay` 1.0)
  (`RitualBottle.SpinBottle` (`self.Bottle`) (`Chair.GetSitter` (`self.Chair1`)) (`Chair.GetSitter` (`self.Chair2`))))

(event `NextTryRitual`
  (bind _lifes (`self.Lifes`))
  (if (`self.bIsFirstAttempt`)
    _
    (elif (<= _lifes 0)
      (`KismetSystemLibrary.PrintString` (`KismetStringLibrary.Conv_IntToString` _lifes))
      (`/Game/_Alex/BP_OuijaBoard.GoodBue` (`self.Board`))
      (else
        (goto _label)))))

(fn `ChooseVictim`)

(fn `UserConstructionScript`)