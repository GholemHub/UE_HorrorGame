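; BP_Room is a puzzle room that rewards bringing a cursed item into the cursed room and closing both its past and future doors.
; It tracks each door's closed state through bound state-change events and whether a BP_Cursed_Item is inside its Box trigger.
; Each door change runs a check that, with both doors closed and the item inside, spawns a key from the item or prints a wrong-room message.
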(event `self.ReceiveBeginPlay`
  (`/Engine/EditorBlueprintResources/StandardMacros.IsValid` (`self.DoorPast`)
    (:`Is Valid`
      (`/Engine/EditorBlueprintResources/StandardMacros.IsValid` (`self.DoorFuture`)
        (:`Is Valid`
          (add `Drag_Item.OnDoorStateChanged` (`self.DoorFuture`) (delegate `OnCloseFuture`))
          (add `Drag_Item.OnDoorStateChanged` (`self.DoorPast`) (delegate `OnClosePast`)))))))

(event `OnClosePast`
  (params (bIsClosed :type Boolean))
  (set `self.Is ClosedP` bIsClosed)
  (`KismetSystemLibrary.PrintString` "Past")
  (`self.OnStartRoomCheck`))

(event `OnCloseFuture`
  (params (bIsClosed :type Boolean))
  (set `self.Is ClosedF` bIsClosed)
  (`KismetSystemLibrary.PrintString` "Future")
  (`self.OnStartRoomCheck`))

(event `self.Box.OnComponentBeginOverlap`
  (params (OverlappedComponent :type "PrimitiveComponent Object Reference") (OtherActor :type "Actor Object Reference") (OtherComp :type "PrimitiveComponent Object Reference") (OtherBodyIndex :type Integer) (bFromSweep :type Boolean) (SweepResult :type "HitResult Structure (by ref)"))
  (bind _asbp_cursed_item (cast `/Game/_Alex/Pickable/BP_Cursed_Item` OtherActor))
  (set `self.As BP Cursed Item` _asbp_cursed_item)
  (set `self.Is CursedInRoom` true))

(event `self.Box.OnComponentEndOverlap`
  (params (OverlappedComponent :type "PrimitiveComponent Object Reference") (OtherActor :type "Actor Object Reference") (OtherComp :type "PrimitiveComponent Object Reference") (OtherBodyIndex :type Integer))
  (cast `/Game/_Alex/Pickable/BP_Cursed_Item` OtherActor)
  (set `self.As BP Cursed Item` null)
  (set `self.Is CursedInRoom` false))

(fn `OnStartRoomCheck`
  (bind _as_bp_cursed_item (`self.As BP Cursed Item`))
  (if (`self.Is ClosedF`)
    (if (`self.Is ClosedP`)
      (if (`self.Is CursedInRoom`)
        (if (`self.CursedRoom`)
          (`/Engine/EditorBlueprintResources/StandardMacros.IsValid` _as_bp_cursed_item
            (:`Is Valid`
              (`/Game/_Alex/Pickable/BP_Cursed_Item.SpawnKey` _as_bp_cursed_item)))
          (else
            (`KismetSystemLibrary.PrintString` "You choose wrong room" true true (struct :`A` 1.0) 5.0)))
        (else
          (`KismetSystemLibrary.PrintString` "Not in room"))))))

(fn `UserConstructionScript`)