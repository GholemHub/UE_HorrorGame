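; BP_Rooms is a room actor that can be cursed and shows the curse through its paintings and a cylinder mesh.
; OnCursedPainting loops over the passed evidence paintings and triggers OnShowCurse on each BP_Paint_Item.
; Tick uses a Delay to check IsCursed about every two seconds and swaps the cylinder's material when true.
; A tentacle reveal for a child painting class and debug prints are left disconnected.
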(event `self.OnCursedPainting`
  (params (EvidencePaintings :type "Array of Actor Object Reference (by ref)"))
  (for _array_element EvidencePaintings
    (bind _asbp_paint_item (cast `/Game/_Alex/Paints/BP_Paint_Item` _array_element))
    (`/Game/_Alex/Paints/BP_Paint_Item.OnShowCurse` _asbp_paint_item)))

(event `self.ReceiveTick`
  (params (DeltaSeconds :type "Float (single-precision)"))
  (`KismetSystemLibrary.Delay` 2.0)
  (if (`self.IsCursed`)
    (`PrimitiveComponent.SetMaterial` (`self.Cylinder`) 0 "/DatasmithContent/Materials/AliasReference.AliasReference")))

(event `self.ReceiveBeginPlay`)

(fn `UserConstructionScript`)