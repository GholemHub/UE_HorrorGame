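; BP_ScareDirector dispatches horror scare events when the player character (HE_CharacterHrono1) overlaps a BP_TriggerBox.
; TriggerFunction switches on the box's gameplay tag to call a light actor's OfLight, turn on the radio, or trigger a demon through a DoOnce.
; The light and demon come from the box's ATriggerActor reference, while the radio is looked up by class.
; The overlap binding is not in this graph.
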(fn `TriggerFunction`
  (params (OverlappedActor :type "Actor Object Reference") (OtherActor :type "Actor Object Reference"))
  (cast `/Game/_Alex/HE_CharacterHrono1` OtherActor)
  (bind _asbp_trigger_box (cast `/Game/_Alex/Room/BP_TriggerBox` OverlappedActor))
  (`|SwitchGameplayTag` (`/Game/_Alex/Room/BP_TriggerBox.TriggerTag` _asbp_trigger_box)
    (:`Trigger.LightPain`
      (bind _atriggeractor (`/Game/_Alex/Room/BP_TriggerBox.ATriggerActor` _asbp_trigger_box))
      (bind _asbp_light_actor (cast `/Game/_Alex/Room/BP_LightActor` _atriggeractor))
      (`/Game/_Alex/Room/BP_LightActor.OfLight` _asbp_light_actor (`local.OtherActor`)))
    (:`Trigger.Radio`
      (bind _returnvalue (`GameplayStatics.GetActorOfClass` "/Game/_Alex/Usable/BP_Radio.BP_Radio_C"))
      (`/Game/_Alex/Usable/BP_Radio.OnRadio` _returnvalue))
    (:`Trigger.Doll`
      (`/Engine/EditorBlueprintResources/StandardMacros.DoOnce` false
        (:`Completed`
          (bind _asbp_demon_1 (cast `/Game/_AI/AI_New/BP_Demon_1` _atriggeractor))
          (`/Game/_AI/AI_New/BP_Demon_1.Trigger` _asbp_demon_1))))))

(fn `UserConstructionScript`)