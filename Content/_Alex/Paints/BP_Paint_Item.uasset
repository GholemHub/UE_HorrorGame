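; BP_Paint_Item is a timeline-aware paint item with curse and scare effects.
; On curse, its hidden meshes and Niagara become scene-capture-only, then it randomly unhides both meshes or activates Niagara; the tentacle event activates Niagara directly.
; While HE_CharacterHrono1 is inside the Sphere, Tick turns both meshes toward that character.
; The scare trigger enables physics on ItemMesh, and OnSameTimeline compares character and item timelines.
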(event `self.ReceiveBeginPlay`
  (`SceneComponent.SetVisibility` (`self.StaticMesh`) false true)
  (`SceneComponent.SetVisibility` (`self.StaticMesh1`) false true)
  (`SceneComponent.SetVisibility` (`self.Niagara`) false true))

(event `OnShowCurse`
  (`PrimitiveComponent.SetVisibleInSceneCaptureOnly` (`self.StaticMesh`) true)
  (`PrimitiveComponent.SetVisibleInSceneCaptureOnly` (`self.StaticMesh1`) true)
  (`PrimitiveComponent.SetVisibleInSceneCaptureOnly` (`self.Niagara`) true)
  (if (`KismetMathLibrary.RandomBool`)
    (`SceneComponent.SetHiddenInGame` (`self.StaticMesh`) false true)
    (`SceneComponent.SetHiddenInGame` (`self.StaticMesh1`) false true)
    (else
      (`ActorComponent.Activate` (`self.Niagara`) true :!label _label))))

(event `OnShowTentacle`
  (goto _label))

(event `self.ReceiveTick`
  (params (DeltaSeconds :type "Float (single-precision)"))
  (bind _as_he_character_hrono_1 (`self.As HE Character Hrono 1`))
  (bind (_returnvalue_x _returnvalue_y _returnvalue_z) (`KismetMathLibrary.BreakVector` (`self.K2_GetActorLocation` _as_he_character_hrono_1)))
  (bind (_returnvalue_roll _returnvalue_pitch _returnvalue_yaw) (`KismetMathLibrary.BreakRotator` (`KismetMathLibrary.FindLookAtRotation` (`SceneComponent.K2_GetComponentLocation` (`self.StaticMesh`)) (`KismetMathLibrary.MakeVector` _returnvalue_x _returnvalue_y (+ _returnvalue_z 60.0)))))
  (bind _returnvalue (+ _returnvalue_pitch 90.0))
  (bind _returnvalue_2 (+ _returnvalue_roll 90.0))
  (`/Engine/EditorBlueprintResources/StandardMacros.IsValid` _as_he_character_hrono_1
    (:`Is Valid`
      (`SceneComponent.K2_SetWorldRotation` (`self.StaticMesh`) (`KismetMathLibrary.MakeRotator` _returnvalue_2 _returnvalue _returnvalue_yaw) false false)
      (`SceneComponent.K2_SetWorldRotation` (`self.StaticMesh1`) (`KismetMathLibrary.MakeRotator` _returnvalue_2 _returnvalue _returnvalue_yaw) false false))))

(event `self.Sphere.OnComponentBeginOverlap`
  (params (OverlappedComponent :type "PrimitiveComponent Object Reference") (OtherActor :type "Actor Object Reference") (OtherComp :type "PrimitiveComponent Object Reference") (OtherBodyIndex :type Integer) (bFromSweep :type Boolean) (SweepResult :type "HitResult Structure (by ref)"))
  (bind _ashe_character_hrono_1 (cast `/Game/_Alex/HE_CharacterHrono1` OtherActor))
  (set `self.As HE Character Hrono 1` _ashe_character_hrono_1))

(event `self.Sphere.OnComponentEndOverlap`
  (params (OverlappedComponent :type "PrimitiveComponent Object Reference") (OtherActor :type "Actor Object Reference") (OtherComp :type "PrimitiveComponent Object Reference") (OtherBodyIndex :type Integer))
  (cast `Character` OtherActor)
  (set `self.As HE Character Hrono 1` null))

(event `/Game/_Alex/I_ScareInterface.OnScareTrigger`
  (params (Triggerer :type "/Game/_Alex/HE_CharacterHrono1 Object Reference"))
  (`PrimitiveComponent.SetSimulatePhysics` (`self.ItemMesh`) true))

(fn `OnSameTimeline`
  (params (CharacterTimeline :type "EItemTimeline Enum" :default "Past"))
  (returns (HasSameTimelines :type Boolean))
  (return (`|EnumEquality` CharacterTimeline (`self.ItemTimeline`))))

(fn `UserConstructionScript`)