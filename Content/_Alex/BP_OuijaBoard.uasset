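; BP_OuijaBoard is a Ouija board word puzzle that mirrors typed letters in VisualText and stages a scare through automatic typing.
; A correct word makes it type "Behind" after a short delay, while GoodBue types "Death".
; When automatic typing finishes, it calls ShowDeath on BP_Chair actors, then, after a delay, plays the dark animation on HE_CharacterHrono1 widgets.
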(event `self.BP_OnTextCancelled`
  (`TextRenderComponent.K2_SetText` (`self.VisualText`) (`self.Value`)))

(event `self.BP_OnTextEntered`
  (params (EnteredText :type String))
  (`TextRenderComponent.K2_SetText` (`self.VisualText`) (`KismetTextLibrary.Conv_StringToText` EnteredText)))

(event `self.ReceiveBeginPlay`
  (add `self.OnNewLetterTyped` (delegate `OnNewLetterTyped_Event`)))

(event `OnNewLetterTyped_Event` :!signature `self.OnNewLetterTyped`
  (params (NewLetter :type String) (FullTypedText :type String))
  (`TextRenderComponent.K2_SetText` (`self.VisualText`) (`KismetTextLibrary.Conv_StringToText` FullTypedText)))

(event `GoodBue`
  (`self.TypeWordAutomatically` "Death" true false))

(event `self.BP_OnCorrectWordEntered`
  (params (CorrectWord :type String))
  (`KismetSystemLibrary.Delay` 1.0)
  (`self.TypeWordAutomatically` "Behind" true false))

(event `self.BP_OnAutomaticTypingFinished`
  (params (Word :type String))
  (`KismetSystemLibrary.Delay` 1.0)
  (bind _outactors (`GameplayStatics.GetAllActorsOfClass` "/Game/_Alex/Usable/BP_Chair.BP_Chair_C"))
  (for _array_element _outactors
    (`/Game/_Alex/Usable/BP_Chair.ShowDeath` _array_element)
    (`KismetSystemLibrary.Delay` 3.0)
    (bind _outactors_2 (`GameplayStatics.GetAllActorsOfClass` "/Game/_Alex/HE_CharacterHrono1.HE_CharacterHrono1_C"))
    (for _array_element_2 _outactors_2
      (bind _wbp_main_char (`/Game/_Alex/HE_CharacterHrono1.WBP_Main_Char` _array_element_2))
      (`/Engine/EditorBlueprintResources/StandardMacros.IsValid` _wbp_main_char
        (:`Is Valid`
          (`/Game/_UI/WBP_Main.PlayAnimDark` _wbp_main_char))))))

(fn `UserConstructionScript`)