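; BP_Babaj is an AI threat actor that kills the player character on contact, unless that character is hiding safely in a wardrobe.
; Its sphere overlap casts to HE_CharacterHrono1, checks the wardrobe safety flag, then calls OnDeath and destroys itself.
; A SetVis event makes the mesh and its children visible, and OnSameTimeline always returns false regardless of the character's timeline.
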(event `Set Vis`
  (`SceneComponent.SetVisibility` (`self.Mesh`) true true))

(event `self.Sphere.OnComponentBeginOverlap`
  (params (OverlappedComponent :type "PrimitiveComponent Object Reference") (OtherActor :type "Actor Object Reference") (OtherComp :type "PrimitiveComponent Object Reference") (OtherBodyIndex :type Integer) (bFromSweep :type Boolean) (SweepResult :type "HitResult Structure (by ref)"))
  (`KismetSystemLibrary.PrintString` "Collision" true true (struct :`R` 0.991771 :`G` 0.957309 :`B` 1.0 :`A` 1.0))
  (bind _ashe_character_hrono_1 (cast `/Game/_Alex/HE_CharacterHrono1` OtherActor))
  (if (not (`HronoCharacter.bIsSafeInHidingWardrobe` _ashe_character_hrono_1))
    (`/Game/_Alex/HE_CharacterHrono1.OnDeath` _ashe_character_hrono_1)
    (`self.K2_DestroyActor`)))

(fn `OnSameTimeline`
  (params (CharacterTimeline :type "EItemTimeline Enum" :default "Past"))
  (returns (HasSameTimelines :type Boolean))
  (return false))

(fn `UserConstructionScript`)