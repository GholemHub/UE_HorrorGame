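; BP_Babaj_Child is a Babaj hazard actor that kills an HE_CharacterHrono1 player entering its sphere, then destroys itself.
; Sphere overlap events set and clear the player's IsInBabajZone flag, with entry leading straight to OnDeath.
; OnChangeStatusSafetie re-triggers the same kill if the player is flagged in the zone, reusing the character cast from the overlap.
; A hiding-wardrobe safety check exists but is disconnected, so entry kills regardless of hiding.
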(event `self.Sphere.OnComponentBeginOverlap`
  (params (OverlappedComponent :type "PrimitiveComponent Object Reference") (OtherActor :type "Actor Object Reference") (OtherComp :type "PrimitiveComponent Object Reference") (OtherBodyIndex :type Integer) (bFromSweep :type Boolean) (SweepResult :type "HitResult Structure (by ref)"))
  (bind _ashe_character_hrono_1 (cast `/Game/_Alex/HE_CharacterHrono1` OtherActor))
  (set `/Game/_Alex/HE_CharacterHrono1.IsInBabajZone` true _ashe_character_hrono_1)
  (`/Game/_Alex/HE_CharacterHrono1.OnDeath` _ashe_character_hrono_1 true :!label _label)
  (`self.K2_DestroyActor`))

(event `self.OnChangeStatusSafetie`
  (params (Player :type "/Game/_Alex/HE_CharacterHrono1 Object Reference"))
  (if (`/Game/_Alex/HE_CharacterHrono1.IsInBabajZone` Player)
    (goto _label)))

(event `self.Sphere.OnComponentEndOverlap`
  (params (OverlappedComponent :type "PrimitiveComponent Object Reference") (OtherActor :type "Actor Object Reference") (OtherComp :type "PrimitiveComponent Object Reference") (OtherBodyIndex :type Integer))
  (bind _ashe_character_hrono_1 (cast `/Game/_Alex/HE_CharacterHrono1` OtherActor))
  (set `/Game/_Alex/HE_CharacterHrono1.IsInBabajZone` false _ashe_character_hrono_1))

(fn `UserConstructionScript`
  (`parent.UserConstructionScript`))