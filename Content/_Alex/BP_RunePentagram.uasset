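; Rune pentagram puzzle actor that controls the darkness threat and Babaj enemies as runes are inserted.
; Showing darkness reveals the DarkDeath actors and toggles their sound, then a delay loop turns each still-visible one into a spawned Babaj child.
; The first and second runes each destroy one Babaj.
; The third clears all Babajs, hides the pentagram, and, per Hrono character, stops the timeline effect, hides darkness and removes rune items.
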(event `self.BP_OnFirstRuneInserted`
  (params (InsertedRune :type "Rune_Item Object Reference") (PlayerWhoInsertedRune :type "HronoCharacter Object Reference") (SlotId :type Name))
  (bind _returnvalue (`GameplayStatics.GetActorOfClass` "/Game/_Alex/AI/BP_Babaj.BP_Babaj_C" :!label _label))
  (`/Engine/EditorBlueprintResources/StandardMacros.IsValid` _returnvalue
    (:`Is Valid`
      (`self.K2_DestroyActor` _returnvalue))))

(event `self.BP_OnSecondRuneInserted`
  (params (InsertedRune :type "Rune_Item Object Reference") (PlayerWhoInsertedRune :type "HronoCharacter Object Reference") (SlotId :type Name))
  (goto _label))

(event `self.BP_OnAllThreeRunesInserted`
  (params (PlayerWhoPlacedLastRune :type "HronoCharacter Object Reference"))
  (`KismetSystemLibrary.PrintString` "THREE 1")
  (bind _outactors (`GameplayStatics.GetAllActorsOfClass` "/Game/_Alex/AI/BP_Babaj.BP_Babaj_C"))
  (for _array_element _outactors
    (`self.K2_DestroyActor` _array_element))
  (`KismetSystemLibrary.PrintString` "NewTime" false false (struct :`R` 0.861522 :`G` 1.0 :`B` 0.903911 :`A` 1.0))
  (`self.SetActorHiddenInGame` true)
  (bind _outactors_2 (`GameplayStatics.GetAllActorsOfClass` "/Game/_Alex/HE_CharacterHrono1.HE_CharacterHrono1_C"))
  (for _array_element_2 _outactors_2
    (`/Game/_Alex/HE_CharacterHrono1.StopSameTimelineEffect` _array_element_2)
    (`self.OnHideDarkness`)
    (bind _outactors_3 (`GameplayStatics.GetAllActorsOfClass` "/Game/_Alex/Pickable/BP_Rune_Item_1.BP_Rune_Item_1_C"))
    (for _array_element_3 _outactors_3
      (`self.K2_DestroyActor` _array_element_3))
    (bind _outactors_4 (`GameplayStatics.GetAllActorsOfClass` "/Game/_Alex/Pickable/BP_Rune_Item_2.BP_Rune_Item_2_C"))
    (for _array_element_4 _outactors_4
      (`self.K2_DestroyActor` _array_element_4))
    (bind _outactors_5 (`GameplayStatics.GetAllActorsOfClass` "/Game/_Alex/Pickable/BP_Rune_Item_3.BP_Rune_Item_3_C"))
    (for _array_element_5 _outactors_5
      (`self.K2_DestroyActor` _array_element_5))))

(event `OnShowDarkness`
  (bind _currentbabajcount (`self.CurrentBabajCount`))
  (bind _darkdeath (`self.DarkDeath`))
  (for _array_element (`self.DarkDeath`)
    (`self.SetActorHiddenInGame` _array_element false)
    (`/Game/_Alex/BP_DarkDeath.On/OffSound` _array_element))
  (`KismetSystemLibrary.Delay` 50.0 :!label _label_2)
  (if (== _currentbabajcount (`KismetArrayLibrary.Array_Length` _darkdeath))
    (`KismetSystemLibrary.PrintString` "END LOOP")
    (else
      (`self.SpawnBabaj` (`|GetArrayItem` _darkdeath _currentbabajcount))
      (set `self.CurrentBabajCount` (+ (`self.CurrentBabajCount`) 1))
      (goto _label_2))))

(event `OnHideDarkness`
  (for _array_element (`self.DarkDeath`)
    (`self.SetActorHiddenInGame` _array_element true)
    (`/Game/_Alex/BP_DarkDeath.On/OffSound` _array_element)))

(fn `SpawnBabaj`
  (params (Dark :type "/Game/_Alex/BP_DarkDeath Object Reference"))
  (if (not (`Actor.bHidden` Dark))
    (`self.SetActorHiddenInGame` Dark true)
    (`AIBlueprintHelperLibrary.SpawnAIFromClass` "/Game/_Alex/AI/BP_Babaj_Child.BP_Babaj_Child_C" null (`SceneComponent.K2_GetComponentLocation` (`/Game/_Alex/BP_DarkDeath.SpawnPoint` Dark)) (struct) false null)))

(fn `UserConstructionScript`)