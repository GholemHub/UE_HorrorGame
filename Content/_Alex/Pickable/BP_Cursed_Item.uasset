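; BP_Cursed_Item is a cursed item actor that can replace itself with a key pickup.
; Its SpawnKey event spawns a BP_Key_Item at the item's location and rotation, enables physics simulation on the key's mesh, then destroys the cursed item.
; The event prints debug strings, and nothing in this Blueprint calls it, so the trigger lives elsewhere.
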(event `SpawnKey`
  (bind _returnvalue (`self.GetTransform`))
  (`KismetSystemLibrary.PrintString` "@!!!!!!!!!!!!!")
  (bind _returnvalue_2 (`|SpawnActorFromClass` "/Game/_Alex/Pickable/BP_Key_Item.BP_Key_Item_C" (`KismetMathLibrary.MakeTransform` (`KismetMathLibrary.MakeVector` (.x (.location _returnvalue)) (.y (.location _returnvalue)) (.z (.location _returnvalue))) (.rotation _returnvalue)) "AlwaysSpawn" "MultiplyWithRoot" null null))
  (`PrimitiveComponent.SetSimulatePhysics` (`Base_Item.ItemMesh` _returnvalue_2) true)
  (`KismetSystemLibrary.PrintString` "Spawned")
  (`self.K2_DestroyActor`))

(fn `UserConstructionScript`
  (`parent.UserConstructionScript`))