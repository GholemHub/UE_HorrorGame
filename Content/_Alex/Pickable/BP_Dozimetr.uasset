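; BP_Dozimetr is a pickable dosimeter that beeps faster the nearer it is to a target actor.
; On starts a beep loop whose delay scales with distance, repeating while it is switched on and its owning character is locally controlled.
; GetClosestActor's search for the nearest Bp_HotDot in the same ItemTimeline is disconnected from the function entry, so it currently supplies no target.
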(event `self.ReceiveOff`
  (set `self.bIsOn` false))

(event `self.ReceiveOn`
  (set `self.bIsOn` true)
  (bind _closestactor (`self.GetClosestActor` :!label _label))
  (`GameplayStatics.PlaySoundAtLocation` "/Game/HorrorEngine/Audio/Elecronics/S_Beep_Dozimetr.S_Beep_Dozimetr" (`self.K2_GetActorLocation`) (struct) 1.0 1.0 0.0 null null null null)
  (`KismetSystemLibrary.Delay` (`KismetMathLibrary.MapRangeClamped` (`KismetMathLibrary.Vector_Distance` (`self.K2_GetActorLocation`) (`self.K2_GetActorLocation` _closestactor)) 20.0 500.0 0.1 2.0))
  (`self.Beep`))

(event `Beep`
  (bind _owningcharacter (`self.OwningCharacter`))
  (`/Engine/EditorBlueprintResources/StandardMacros.IsValid` _owningcharacter
    (:`Is Valid`
      (if (and (`self.bIsOn`) (`Pawn.IsLocallyControlled` _owningcharacter))
        (goto _label)))))

(fn `GetClosestActor`
  (returns (ClosestActor :type "Actor Object Reference")))

(fn `UserConstructionScript`)