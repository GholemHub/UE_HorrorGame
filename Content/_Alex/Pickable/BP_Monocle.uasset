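; BP_Monocle is a pickable monocle with a SceneCaptureComponent2D that runs only while the item is held.
; The capture component is deactivated on BeginPlay.
; OnHeldStateChanged reads IsPickedUp to activate the capture with a reset on pickup and deactivate it otherwise.
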(event `self.ReceiveBeginPlay`
  (`ActorComponent.Deactivate` (`self.SceneCaptureComponent2D`)))

(event `self.OnHeldStateChanged`
  (params (bIsHeld :type Boolean) (Character :type "HronoCharacter Object Reference"))
  (bind _scenecapturecomponent2d (`self.SceneCaptureComponent2D`))
  (if (`self.bIsPickedUp`)
    (`ActorComponent.Activate` _scenecapturecomponent2d true)
    (else
      (`ActorComponent.Deactivate` _scenecapturecomponent2d))))

(fn `UserConstructionScript`)