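; BP_Item_Bottle_Roulette is a bottle item for a spin-the-bottle roulette, apparently still in prototype.
; The Fall event takes a spin value and runs a timeline that scales it into the mesh's physics angular velocity around Z.
; Two seconds after the timeline ends, ChooseVictim only debug-prints the absolute yaw and whether it reaches 90 degrees.
; A SpinCounter RepNotify turns off physics simulation, while the TargetBottleRotation RepNotify is empty.
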(event `Fall`
  (params (Rand :type "Float (double-precision)"))
  (set `self.SpinDegrees` Rand)
  (`KismetSystemLibrary.PrintString` (`KismetStringLibrary.Concat_StrStr` "Random:::::" (`KismetStringLibrary.Conv_DoubleToString` (`self.SpinDegrees`))) true true (struct :`G` 0.66 :`B` 1.0 :`A` 1.0) 10.0)
  (bind (_direction _newtrack_0) (`Timeline|Timeline` :!via `PlayFromStart`)
    (:`Update`
      (`PrimitiveComponent.SetPhysicsAngularVelocityInDegrees` (`self.StaticMesh`) (`KismetMathLibrary.MakeVector` 0.0 0.0 (* _newtrack_0 (`self.SpinDegrees`))) false "None"))
    (:`Finished`
      (`KismetSystemLibrary.PrintString` "Hello")
      (`KismetSystemLibrary.Delay` 2.0)
      (`self.ChooseVictim`))))

(fn `ChooseVictim`
  (bind (_returnvalue_roll _returnvalue_pitch _returnvalue_yaw) (`KismetMathLibrary.BreakRotator` (`SceneComponent.K2_GetComponentRotation` (`self.StaticMesh`))))
  (bind _returnvalue (`KismetMathLibrary.Abs` (`KismetMathLibrary.NormalizeAxis` _returnvalue_yaw)))
  (`KismetSystemLibrary.PrintString` (`KismetStringLibrary.Concat_StrStr` "Delta:::::" (`KismetStringLibrary.Conv_DoubleToString` _returnvalue) "Mirror" (`KismetStringLibrary.Conv_BoolToString` (>= _returnvalue 90.0))) true true (struct :`R` 1.0 :`B` 0.451097 :`A` 1.0) 10.0))

(fn `OnRep_SpinCounter`
  (`PrimitiveComponent.SetSimulatePhysics` (`self.StaticMesh`) false))

(fn `OnRep_TargetBottleRotation`)

(fn `UserConstructionScript`
  (`parent.UserConstructionScript`))