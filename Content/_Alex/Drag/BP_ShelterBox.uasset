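; BP_ShelterBox is a shelter trigger volume that reacts to the HE_CharacterHrono1 character entering and leaving its Box.
; On entry it prints "SAVE", creates and stores a dynamic material instance from the DoorToHide mesh's first material, and sets its Opacity parameter.
; On exit it prints "Unsave" and sets Opacity to the same fully opaque value, so the door gets no different fade state.
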(event `self.Box.OnComponentBeginOverlap`
  (params (OverlappedComponent :type "PrimitiveComponent Object Reference") (OtherActor :type "Actor Object Reference") (OtherComp :type "PrimitiveComponent Object Reference") (OtherBodyIndex :type Integer) (bFromSweep :type Boolean) (SweepResult :type "HitResult Structure (by ref)"))
  (bind _itemmesh (`Base_Item.ItemMesh` (`self.DoorToHide`)))
  (cast `/Game/_Alex/HE_CharacterHrono1` OtherActor)
  (`KismetSystemLibrary.PrintString` "SAVE")
  (bind _returnvalue (`PrimitiveComponent.CreateDynamicMaterialInstance` _itemmesh 0 (`PrimitiveComponent.GetMaterial` _itemmesh 0) "None"))
  (bind _output_get (set `self.MaterialOpacity` _returnvalue))
  (`MaterialInstanceDynamic.SetScalarParameterValue` _output_get "Opacity" 1.0))

(event `self.Box.OnComponentEndOverlap`
  (params (OverlappedComponent :type "PrimitiveComponent Object Reference") (OtherActor :type "Actor Object Reference") (OtherComp :type "PrimitiveComponent Object Reference") (OtherBodyIndex :type Integer))
  (cast `/Game/_Alex/HE_CharacterHrono1` OtherActor)
  (`KismetSystemLibrary.PrintString` "Unsave")
  (`MaterialInstanceDynamic.SetScalarParameterValue` (`self.MaterialOpacity`) "Opacity" 1.0))

(fn `UserConstructionScript`)